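; BP_Weapon is an inventory weapon item that, when its box overlaps a ground animal, temporarily scares that animal off.
; The overlap switches the animal from Harass to RunAway, then one shared Delay reverses both flags after twenty seconds.
; Dropped stores the item ID, calls CreateItem and applies ThisMesh to the static mesh component.
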(event `self.Box.OnComponentBeginOverlap`
  (params (OverlappedComponent :type "PrimitiveComponent Object Reference") (OtherActor :type "Actor Object Reference") (OtherComp :type "PrimitiveComponent Object Reference") (OtherBodyIndex :type Integer) (bFromSweep :type Boolean) (SweepResult :type "HitResult Structure (by ref)"))
  (bind _asbp_ground_animal_base (cast `/Game/AnimalBehaviorKit/Animals/GroundAnimals/BP_GroundAnimalBase` OtherActor))
  (set `AnimalBase.RunAway` true _asbp_ground_animal_base)
  (set `GroundAnimalBase.Harass` false _asbp_ground_animal_base)
  (`KismetSystemLibrary.Delay` 20.0)
  (set `AnimalBase.RunAway` false _asbp_ground_animal_base)
  (set `GroundAnimalBase.Harass` true _asbp_ground_animal_base))

(fn `Dropped`
  (params (ID :type Integer))
  (set `self.ItemID` ID)
  (`self.CreateItem`)
  (`self.MakeMeshCorrect`))

(fn `MakeMeshCorrect`
  (`StaticMeshComponent.SetStaticMesh` (`self.StaticMeshComponent`) (`self.ThisMesh`)))

(fn `UserConstructionScript`
  (`parent.UserConstructionScript`))